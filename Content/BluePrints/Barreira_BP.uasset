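; Player-raised barrier that spends collected skulls (Caveiras) to block aliens.
; On the Formar Barreira input, with enough skulls, it zeroes the count, plays a sound, briefly shows an animated Death figure and raises Cube and Box with MoveComponentTo.
; Each Alien_01 overlap on Box reduces Health.
; At zero Health the barrier sinks, resets its Health and can be raised again.
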(event OnComponentBeginOverlap(Box)
  (params (OverlappedComponent :type Primitive%20Component%20Object%20Reference) (OtherActor :type Actor%20Object%20Reference) (OtherComp :type Primitive%20Component%20Object%20Reference) (OtherBodyIndex :type Integer) (bFromSweep :type Boolean) (SweepResult :type Hit%20Result%20Structure%20%28by%20ref%29))
  (bind _cube (Variables|Default|GetCube))
  (bind _box (Variables|Default|GetBox))
  (bind _returnvalue (Transformation|GetRelativeTransform _cube))
  (bind _returnvalue_2 (Transformation|GetRelativeTransform _box))
  (Utilities|Casting|CastToAlien_01 OtherActor)
  (Variables|Default|Sethealth (- (Variables|Default|Gethealth) (Variables|Default|GetDano%20do%20tiro%20do%20alien)))
  (if (<= (Variables|Default|Gethealth) 0.0)
    (Variables|Default|SetFeita false)
    (Components|MoveComponentTo _cube (Math|Vector|MakeVector (.x (.location _returnvalue)) (.y (.location _returnvalue)) -75.0) (.rotation _returnvalue) false true 2.0 false)
    (Components|MoveComponentTo _box (Math|Vector|MakeVector (.x (.location _returnvalue_2)) (.y (.location _returnvalue_2)) -75.0) (.rotation _returnvalue_2) false true 1.0 false)
    (Variables|Default|Sethealth 1e+02)))

(event EventBeginPlay)

(event Collision|EventActorBeginOverlap
  (params (OtherActor :type Actor%20Object%20Reference)))

(event EventTick
  (params (DeltaSeconds :type Float%20%28single-precision%29)))

(event Input|ActionEvents|InputActionFormarBarreira
  (params (Key :type Key%20Structure))
  (bind _jogador (Variables|Default|GetJogador))
  (bind _cube (Variables|Default|GetCube))
  (bind _box (Variables|Default|GetBox))
  (bind _returnvalue (Transformation|GetRelativeTransform _cube))
  (bind _returnvalue_2 (Transformation|GetRelativeTransform _box))
  (:Pressed
    (if (not (Variables|Default|GetFeita))
      (if (>= (Variables|/Game/BluePrints/Jogador.Jogador_C|GetCaveiras _jogador) 8.0)
        (Variables|/Game/BluePrints/Jogador.Jogador_C|SetCaveiras _jogador 0.0)
        (Audio|PlaySound2D "/Game/SFX/Transmutação_Cue.Transmutação_Cue")
        (Development|SetHiddeninGame (Variables|Default|GetDeath) false false)
        (Components|Animation|PlayAnimation (Variables|Default|GetDeath) "/Game/Animações/Death_Magic_Attack.Death_Magic_Attack" true)
        (Components|MoveComponentTo _cube (Math|Vector|MakeVector (.x (.location _returnvalue)) (.y (.location _returnvalue)) 75.0) (.rotation _returnvalue) false true 1.0 false)
        (Variables|Default|SetFeita true)
        (Components|MoveComponentTo _box (Math|Vector|MakeVector (.x (.location _returnvalue_2)) (.y (.location _returnvalue_2)) 75.0) (.rotation _returnvalue_2) false true 1.0 false)
        (Utilities|FlowControl|Delay 2.0)
        (Development|SetHiddeninGame (Variables|Default|GetDeath) true false)))))

(fn ConstructionScript)