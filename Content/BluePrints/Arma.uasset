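; Weapon Blueprint that spawns hero projectiles (ProjetilDoHeroi) at its SpawnPoint transform.
; PullTrigger passes through a DoOnce to fire immediately, then sets a timer at an interval derived from TirosPorSegundo (shots per second).
; ReleaseTrigger calls clear timer and resets the DoOnce for the next pull.
; The timer nodes name no function, so repeat fire is not wired to Fire.
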(event Custom|Pull%20Trigger
  (Utilities|FlowControl|DoOnce false
    (:Completed
      (CallFunction|Fire)
      (Utilities|Time|SetTimerbyFunctionName 0 "" (/ 1.0 (Variables|Default|GetTiros%20por%20Segundo))))))

(event Custom|Release%20Trigger
  (Utilities|Time|ClearTimerbyFunctionName 0 "")
  (Utilities|FlowControl|DoOnce false) ; enters at Reset
)

(event Custom|Fire
  (Game|SpawnActorfromClass "/Game/BluePrints/ProjetilDoHeroi.ProjetilDoHeroi_C" (Transformation|GetWorldTransform (Variables|Default|GetSpawn%20Point)) "Undefined" 0 0))

(event EventBeginPlay)

(event Collision|EventActorBeginOverlap
  (params (OtherActor :type Actor%20Object%20Reference)))

(event EventTick
  (params (DeltaSeconds :type Float%20%28single-precision%29)))

(fn ConstructionScript)