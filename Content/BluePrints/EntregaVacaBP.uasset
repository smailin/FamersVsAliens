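; Cow-delivery actor that plays an abduction sequence, raising a barn after the Alien_01 actor enters its box trigger.
; Overlap reveals four legs and a spotlight, lowers the legs, then after a delay sets a flag that makes Tick lift the barn.
; Leaving the box retracts and hides them.
; Tick also calls that retraction whenever the lift flag is off after activation, including during the delay; Enter clears the flag.
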(event OnComponentBeginOverlap(Box)
  (params (OverlappedComponent :type Primitive%20Component%20Object%20Reference) (OtherActor :type Actor%20Object%20Reference) (OtherComp :type Primitive%20Component%20Object%20Reference) (OtherBodyIndex :type Integer) (bFromSweep :type Boolean) (SweepResult :type Hit%20Result%20Structure%20%28by%20ref%29))
  (Utilities|Casting|CastToAlien_01 OtherActor
    (:then
      (CallFunction|Abduzir))
    (:CastFailed
      (Variables|Default|SetAbduzindo false))))

(event OnComponentEndOverlap(Box)
  (params (OverlappedComponent :type Primitive%20Component%20Object%20Reference) (OtherActor :type Actor%20Object%20Reference) (OtherComp :type Primitive%20Component%20Object%20Reference) (OtherBodyIndex :type Integer))
  (Utilities|Casting|CastToAlien_01 OtherActor
    (:then
      (CallFunction|RecolhaPernas))
    (:CastFailed
      (Variables|Default|SetAbduzindo false))))

(event Custom|Abduzir
  (bind _perna01 (Variables|Default|GetPerna01))
  (bind _perna03 (Variables|Default|GetPerna03))
  (bind _perna02 (Variables|Default|GetPerna02))
  (bind _perna04 (Variables|Default|GetPerna04))
  (bind _returnvalue (Transformation|GetRelativeTransform _perna01))
  (bind _returnvalue_2 (Transformation|GetRelativeTransform _perna02))
  (bind _returnvalue_3 (Transformation|GetRelativeTransform _perna03))
  (bind _returnvalue_4 (Transformation|GetRelativeTransform _perna04))
  (Variables|Default|Setanimando true)
  (Development|SetHiddeninGame (Variables|Default|GetPerna02) false false)
  (Components|MoveComponentTo _perna01 (Math|Vector|MakeVector (.x (.location _returnvalue)) (.y (.location _returnvalue)) 0.0) (.rotation _returnvalue) false false 1.0 false)
  (Components|MoveComponentTo _perna02 (Math|Vector|MakeVector (.x (.location _returnvalue_2)) (.y (.location _returnvalue_2)) 0.0) (.rotation _returnvalue_2) false false 1.0 false)
  (Components|MoveComponentTo _perna03 (Math|Vector|MakeVector (.x (.location _returnvalue_3)) (.y (.location _returnvalue_3)) 0.0) (.rotation _returnvalue_3) false false 1.0 false)
  (Components|MoveComponentTo _perna04 (Math|Vector|MakeVector (.x (.location _returnvalue_4)) (.y (.location _returnvalue_4)) 0.0) (.rotation _returnvalue_4) false false 1.0 false)
  (Utilities|FlowControl|Delay 13.0)
  (Variables|Default|SetAbduzindo true))

(event Custom|Cutscene
  (Components|MoveComponentTo (Variables|Default|GetBarn) "0.0,0.0,500.000000" "0, 0, 0" false false 1e+01 false))

(event Custom|Recolha%20pernas
  (bind _perna02 (Variables|Default|GetPerna02))
  (bind _perna03 (Variables|Default|GetPerna03))
  (bind _perna04 (Variables|Default|GetPerna04))
  (bind _perna01 (Variables|Default|GetPerna01))
  (bind _returnvalue (Transformation|GetRelativeTransform _perna02))
  (bind _returnvalue_2 (Transformation|GetRelativeTransform _perna03))
  (bind _returnvalue_3 (Transformation|GetRelativeTransform _perna04))
  (bind _returnvalue_4 (Transformation|GetRelativeTransform _perna01))
  (Components|MoveComponentTo _perna01 (Math|Vector|MakeVector (.x (.location _returnvalue_4)) (.y (.location _returnvalue_4)) 1e+03) (.rotation _returnvalue_4) false false 1.0 false)
  (Components|MoveComponentTo _perna02 (Math|Vector|MakeVector (.x (.location _returnvalue)) (.y (.location _returnvalue)) 1e+03) (.rotation _returnvalue) false false 1.0 false)
  (Components|MoveComponentTo _perna03 (Math|Vector|MakeVector (.x (.location _returnvalue_2)) (.y (.location _returnvalue_2)) 1e+03) (.rotation _returnvalue_2) false false 1.0 false)
  (Components|MoveComponentTo _perna04 (Math|Vector|MakeVector (.x (.location _returnvalue_3)) (.y (.location _returnvalue_3)) 1e+03) (.rotation _returnvalue_3) false false 1.0 false)
  (Development|SetHiddeninGame (Variables|Default|GetPerna02) true false))

(event EventBeginPlay
  (Variables|Default|SetAbduzindo false))

(event Collision|EventActorBeginOverlap
  (params (OtherActor :type Actor%20Object%20Reference)))

(event EventTick
  (params (DeltaSeconds :type Float%20%28single-precision%29))
  (if (Variables|Default|GetAbduzindo)
    (CallFunction|Cutscene)
    (elif (Variables|Default|Getanimando)
      (CallFunction|RecolhaPernas))))

(event Input|KeyboardEvents|Enter
  (params (Key :type Key%20Structure))
  (:Pressed
    (Variables|Default|SetAbduzindo false)))

(fn ConstructionScript)